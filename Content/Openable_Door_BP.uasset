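; Openable door actor that swings open and closed when its OpenDoor component broadcasts open and close requests.
; It caches its starting rotation at BeginPlay, then a timeline plays or reverses to add a yaw offset to that rotation each update.
; An event track on the same timeline plays a door lock sound at the actor's location.
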(event OnOpenRequest(OpenDoor)
  (bind _rotation (Timeline|Timeline_0 Play)
    (:Update
      (Transformation|SetActorRotation (Math|Rotator|CombineRotators (Variables|Default|GetStartRotation) (Math|Rotator|MakeRotator 0.0 0.0 _rotation))))
    (:Sound
      (Audio|PlaySoundatLocation "/Game/door-lock.door-lock" (Transformation|GetActorLocation) "0, 0, 0" 1.0 1.0 0.0 0 0 0))))

(event OnCloseRequest(OpenDoor)
  (bind _rotation (Timeline|Timeline_0 Reverse)
    (:Update
      (Transformation|SetActorRotation (Math|Rotator|CombineRotators (Variables|Default|GetStartRotation) (Math|Rotator|MakeRotator 0.0 0.0 _rotation))))
    (:Sound
      (Audio|PlaySoundatLocation "/Game/door-lock.door-lock" (Transformation|GetActorLocation) "0, 0, 0" 1.0 1.0 0.0 0 0 0))))

(event EventBeginPlay
  (Variables|Default|SetStartRotation (Transformation|GetActorRotation)))

(fn ConstructionScript)